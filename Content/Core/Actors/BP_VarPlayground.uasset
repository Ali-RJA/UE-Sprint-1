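; BP_VarPlayground is a test actor that spawns and destroys actors from keyboard input, driven by its class, offset and reference variables.
; Key 1 spawns TargetClass at the actor's location plus SpawnOffset, stores it in LastSpawned and shows its name in StatusText.
; Key 2 destroys LastSpawned after a validity check.
; BeginPlay prints the offset and shows the target class name in StatusText.
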(event `Key|One`
  (params (Key :type "Key Structure"))
  (:`Pressed`
    (bind _returnvalue (`|SpawnActorFromClass` (`self.TargetClass`) (`KismetMathLibrary.MakeTransform` (+ (`self.SpawnOffset`) (`self.K2_GetActorLocation`))) "Undefined" "MultiplyWithRoot" null null))
    (bind _output_get (set `self.LastSpawned` _returnvalue))
    (`TextRenderComponent.K2_SetText` (`self.StatusText`) (`KismetTextLibrary.Conv_StringToText` (`KismetSystemLibrary.GetDisplayName` _output_get)))))

(event `Key|Two`
  (params (Key :type "Key Structure"))
  (bind _lastspawned (`self.LastSpawned`))
  (:`Pressed`
    (`KismetSystemLibrary.IsValid` _lastspawned)
    (`self.K2_DestroyActor` _lastspawned)))

(event `self.ReceiveBeginPlay`
  (`KismetSystemLibrary.PrintString` (`KismetStringLibrary.Conv_VectorToString` (`self.SpawnOffset`)))
  (`TextRenderComponent.K2_SetText` (`self.StatusText`) (`KismetTextLibrary.Conv_StringToText` (`KismetSystemLibrary.GetClassDisplayName` (`self.TargetClass`)))))

(fn `UserConstructionScript`)